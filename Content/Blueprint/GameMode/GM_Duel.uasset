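; GM_Duel is the game mode for a samurai quick-draw duel between a player and an NPC.
; Tick advances the phase from Intro to Wait, then after a random delay to Draw, signalling it, showing an exclamation actor and starting a restart-delay timer.
; A successful attack defeats the opposing samurai and hides the exclamation.
; Separate functions mark the duel finished or reset the phase, elapsed time and both samurai.
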(event `self.ReceiveBeginPlay`
  (bind _returnvalue (`GameplayStatics.GetActorOfClass` "/Game/Blueprint/BP_exclamation.BP_exclamation_C"))
  (set `self.Exclamation Ref` _returnvalue)
  (bind _returnvalue_2 (`GameplayStatics.GetActorOfClass` "/Game/Blueprint/BP_Samurai_Player.BP_Samurai_Player_C"))
  (set `self.Samurai Player` _returnvalue_2)
  (bind _returnvalue_3 (`GameplayStatics.GetActorOfClass` "/Game/Blueprint/BP_Samurai_NPC.BP_Samurai_NPC_C"))
  (set `self.SamuraiNPC` _returnvalue_3))

(event `self.ReceiveTick`
  (params (DeltaSeconds :type "Float (single-precision)"))
  (set `self.ElapsedTime` (+ DeltaSeconds (`self.ElapsedTime`)))
  (switch `/Game/Blueprint/Enums/E_Phase` (`self.Phase`)
    (:`NewEnumerator0`
      (if (> (`self.ElapsedTime`) (`self.RoundStartTime`))
        (set `self.Phase` "NewEnumerator1")
        (`KismetSystemLibrary.Delay` (`KismetMathLibrary.RandomFloatInRange` (`self.MinDrawDeleay`) (`self.MaxDrawDelay`)))
        (set `self.Phase` "NewEnumerator2")
        (`self.DrawPhaseStarted`)
        (`/Engine/EditorBlueprintResources/StandardMacros.IsValid` (`self.Exclamation Ref`)
          (:`Is Valid`
            (`/Game/Blueprint/BP_exclamation.SetVisibility` (`self.Exclamation Ref`) true)
            (`KismetSystemLibrary.K2_SetTimerDelegate` (`|CreateDelegate` :!event `ResetGameMode`) (`self.RestartDelay`))))))))

(fn `AttackedSuccscesfully`
  (params (`Is Player` :type Boolean))
  (if `Is Player`
    (`/Game/Blueprint/BP_Samurai.Defeated` (`self.SamuraiNPC`))
    (else
      (`/Game/Blueprint/BP_Samurai.Defeated` (`self.Samurai Player`))))
  (`/Engine/EditorBlueprintResources/StandardMacros.IsValid` (`self.Exclamation Ref`)
    (:`Is Valid`
      (`/Game/Blueprint/BP_exclamation.SetVisibility` (`self.Exclamation Ref`) false))))

(fn `ResetGameMode`
  (set `self.Phase` "NewEnumerator0")
  (set `self.ElapsedTime` 0.0)
  (`/Game/Blueprint/BP_Samurai.ResetSamurai` (`self.Samurai Player`))
  (`/Game/Blueprint/BP_Samurai.ResetSamurai` (`self.SamuraiNPC`)))

(fn `SetGameFinisched`
  (set `self.Phase` "NewEnumerator3"))

(fn `UserConstructionScript`)