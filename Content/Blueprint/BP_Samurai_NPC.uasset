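; Samurai NPC Blueprint that automatically attacks during the game's draw phase.
; On BeginPlay it runs the parent logic and binds a handler to the GameMode's draw-phase-started event.
; When that event fires, it waits a random time between the minimum and maximum attack delays, then calls Attack.
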(event `self.ReceiveBeginPlay`
  (`parent.ReceiveBeginPlay`)
  (add `/Game/Blueprint/GameMode/GM_Duel.DrawPhaseStarted` (`self.GameMode`) (delegate `OnDrawPhaseStarted`)))

(event `OnDrawPhaseStarted`
  (`KismetSystemLibrary.Delay` (`KismetMathLibrary.RandomFloatInRange` (`self.MinDelayAttack`) (`self.MaxDelayAttack`)))
  (`self.Attack`))

(fn `UserConstructionScript`
  (`parent.UserConstructionScript`))